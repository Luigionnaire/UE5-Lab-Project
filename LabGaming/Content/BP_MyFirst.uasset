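; BP_MyFirst is a Blueprint that exercises basic arithmetic functions and shows their results on screen, with no other gameplay logic.
; On BeginPlay it calls MyFunction, then add, subtract, divide and multiply functions with constant inputs, none of which are defined in this file.
; The four results are converted to strings, concatenated without separators and shown through a single PrintString.
; Overlap, Tick and the construction script are empty.
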(event EventBeginPlay
  (Class|MyFirst|MyFunction)
  (bind _returnvalue (Class|MyFirst|AddNumbers 1.0 1.0))
  (bind _returnvalue_2 (Class|MyFirst|SubtractNumbers 4.0 2.0))
  (bind _returnvalue_3 (Class|MyFirst|DivideNumbers 4.0 2.0))
  (bind _returnvalue_4 (Class|MyFirst|MultiplyNumbers 2.0 1.0))
  (Development|PrintString (Utilities|String|Append (Utilities|String|Append (Utilities|String|Append (Utilities|String|ToString(Float) _returnvalue) (Utilities|String|ToString(Float) _returnvalue_2)) (Utilities|String|ToString(Float) _returnvalue_3)) (Utilities|String|ToString(Float) _returnvalue_4)) true true "(R=0.000000,G=0.660000,B=1.000000,A=1.000000)" 1e+01))

(event Collision|EventActorBeginOverlap
  (params (OtherActor :type Actor%20Object%20Reference)))

(event EventTick
  (params (DeltaSeconds :type Float%20%28single-precision%29)))

(fn ConstructionScript)